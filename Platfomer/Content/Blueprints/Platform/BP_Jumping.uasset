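; BP_Jumping is a platform Blueprint that boosts the player's jump while they are inside its Trigger volume.
; On begin overlap it caches the BP_Player's JumpZVelocity and sets it to one and a half times that value.
; On end overlap it restores the player's velocity from that single cached variable.
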(event `self.Trigger.OnComponentBeginOverlap`
  (params (OverlappedComponent :type "PrimitiveComponent Object Reference") (OtherActor :type "Actor Object Reference") (OtherComp :type "PrimitiveComponent Object Reference") (OtherBodyIndex :type Integer) (bFromSweep :type Boolean) (SweepResult :type "HitResult Structure (by ref)"))
  (bind _asbp_player (cast `/Game/Blueprints/BP_Player` OtherActor))
  (bind _charactermovement (`Character.CharacterMovement` _asbp_player))
  (bind _output_get (set `self.OriginJumpZVelocity` (`CharacterMovementComponent.JumpZVelocity` _charactermovement)))
  (set `CharacterMovementComponent.JumpZVelocity` (* _output_get 1.5) _charactermovement))

(event `self.Trigger.OnComponentEndOverlap`
  (params (OverlappedComponent :type "PrimitiveComponent Object Reference") (OtherActor :type "Actor Object Reference") (OtherComp :type "PrimitiveComponent Object Reference") (OtherBodyIndex :type Integer))
  (bind _asbp_player (cast `/Game/Blueprints/BP_Player` OtherActor))
  (set `CharacterMovementComponent.JumpZVelocity` (`self.OriginJumpZVelocity`) (`Character.CharacterMovement` _asbp_player)))

(fn `UserConstructionScript`
  (`parent.UserConstructionScript`))