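; BP_Moving is a moving platform that shuttles back and forth between its starting position and an EndPoint marker.
; BeginPlay caches the direction and distance to the marker, then hides it in game.
; Tick moves PlatformMesh by Speed every frame without sweep or delta-time scaling, so movement is frame-rate dependent.
; It reverses direction whenever the accumulated travel exceeds the distance, without snapping to either endpoint.
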(event `self.ReceiveBeginPlay`
  (bind _endpoint (`self.EndPoint`))
  (bind _returnvalue (- (`self.End`) (`self.Start`)))
  ; BeginPlay
  (`parent.ReceiveBeginPlay`)
  (set `self.Start` (`SceneComponent.K2_GetComponentLocation` (`self.PlatformMesh`)))
  (set `self.End` (`SceneComponent.K2_GetComponentLocation` _endpoint))
  (set `self.Distance` (`KismetMathLibrary.VSize` _returnvalue))
  (set `self.Direction` (`KismetMathLibrary.Normal` _returnvalue))
  (`SceneComponent.SetHiddenInGame` _endpoint true false))

(event `self.ReceiveTick`
  (params (DeltaSeconds :type "Float (single-precision)"))
  ; Tick
  (`parent.ReceiveTick` DeltaSeconds)
  (`|ExecutionSequence`
    (:`then_0`
      (`SceneComponent.K2_SetWorldLocation` (`self.PlatformMesh`) (+ (`SceneComponent.K2_GetComponentLocation` (`self.PlatformMesh`)) (* (`self.Direction`) (`self.Speed`))) false false))
    (:`then_1`
      (bind _output_get (set `self.MoveDistance` (+ (`self.MoveDistance`) (`self.Speed`))))
      (if (> _output_get (`self.Distance`))
        (set `self.Direction` (* (`self.Direction`) (`KismetMathLibrary.Conv_DoubleToVector` -1.0)))
        (set `self.MoveDistance` 0.0)))))

(fn `UserConstructionScript`
  (`parent.UserConstructionScript`))