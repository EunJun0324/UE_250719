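; BP_Player is the player pawn or character, with Enhanced Input movement, look and jump, a three-heart health system, and Escape to quit.
; BeginPlay adds the input mapping and creates the WBP_Player HUD.
; Any damage teleports the player to a PlayerStart and decrements Hp, while a timeline animates the heart's removal, then triggers the widget's GameOver at zero.
; The interact input is an empty stub.
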(event `self.ReceiveBeginPlay`
  (bind `_as플레이어_컨트롤러` (cast `PlayerController` (`self.GetController`)))
  (`EnhancedInputSubsystemInterface.AddMappingContext` (pcsubsystem `EnhancedInputLocalPlayerSubsystem` `_as플레이어_컨트롤러`) "/Game/Blueprints/Inputs/IMC_Player.IMC_Player" 0 (struct))
  (bind _returnvalue (`|CreateWidget` "/Game/Blueprints/Widgets/WBP_Player.WBP_Player_C"))
  (bind _output_get (set `self.PlayerWidget` _returnvalue))
  (`UserWidget.AddToViewport` _output_get 0)
  (set `self.Hp` 3))

(event `EnhancedInput|/Game/Blueprints/Inputs/IA_Move`
  (params (ActionValue :type "Vector2D Structure") (ElapsedSeconds :type "Float (double-precision)") (TriggeredSeconds :type "Float (double-precision)") (InputAction :type "InputAction Object Reference" :default "/Game/Blueprints/Inputs/IA_Move.IA_Move"))
  (:`Triggered`
    (`self.AddMovementInput` (`self.GetActorForwardVector`) ActionValue_X)
    (`self.AddMovementInput` (`self.GetActorRightVector`) ActionValue_Y)))

(event `EnhancedInput|/Game/Blueprints/Inputs/IA_Look`
  (params (ActionValue :type "Vector2D Structure") (ElapsedSeconds :type "Float (double-precision)") (TriggeredSeconds :type "Float (double-precision)") (InputAction :type "InputAction Object Reference" :default "/Game/Blueprints/Inputs/IA_Look.IA_Look"))
  (:`Triggered`
    (`self.AddControllerYawInput` ActionValue_X)
    (`self.AddControllerPitchInput` ActionValue_Y)))

(event `EnhancedInput|/Game/Blueprints/Inputs/IA_Jump`
  (params (ActionValue :type Boolean) (ElapsedSeconds :type "Float (double-precision)") (TriggeredSeconds :type "Float (double-precision)") (InputAction :type "InputAction Object Reference" :default "/Game/Blueprints/Inputs/IA_Jump.IA_Jump"))
  (:`Started`
    (`self.Jump`)))

(event `Key|Escape`
  (params (Key :type "Key Structure"))
  (:`Pressed`
    (`KismetSystemLibrary.QuitGame` null "Quit")))

(event `EnhancedInput|/Game/Blueprints/Inputs/IA_Interact`
  (params (ActionValue :type Boolean) (ElapsedSeconds :type "Float (double-precision)") (TriggeredSeconds :type "Float (double-precision)") (InputAction :type "InputAction Object Reference" :default "/Game/Blueprints/Inputs/IA_Interact.IA_Interact")))

(event `self.ReceiveAnyDamage`
  (params (Damage :type "Float (single-precision)") (DamageType :type "DamageType Object Reference") (InstigatedBy :type "Controller Object Reference") (DamageCauser :type "Actor Object Reference"))
  (bind _playerwidget (`self.PlayerWidget`))
  (`self.K2_SetActorLocation` (`self.K2_GetActorLocation` (`GameModeBase.K2_FindPlayerStart` (`GameplayStatics.GetGameMode`) (`self.GetController`) "")))
  (bind _result (`/Engine/EditorBlueprintResources/StandardMacros.DecrementInt` (`self.Hp`))
    (:`  `
      (bind (_direction _alpha) (`Timeline|타임라인` :!via `PlayFromStart`)
        (:`Update`
          (`/Game/Blueprints/Widgets/WBP_Player.RemoveHeart` _playerwidget (`KismetMathLibrary.Clamp` _result 0 3) _alpha))
        (:`Finished`
          (if (== (`self.Hp`) 0)
            (`/Game/Blueprints/Widgets/WBP_Player.GameOver` _playerwidget)))))))

(fn `UserConstructionScript`)